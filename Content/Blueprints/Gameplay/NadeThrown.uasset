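; Thrown grenade actor, launched along a configurable local velocity by projectile movement, that explodes after a fixed delay once its mesh hits something.
; Hits route through an authority switch to a shared detonation event, with no guard against repeat hits.
; Detonation spawns an explosion emitter and timed burn mark, damages characters overlapping the sphere with clamped linear distance falloff, then destroys the actor.
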(event `self.ReceiveBeginPlay`)

(event `self.StaticMesh.OnComponentHit`
  (params (HitComponent :type "PrimitiveComponent Object Reference") (OtherActor :type "Actor Object Reference") (OtherComp :type "PrimitiveComponent Object Reference") (NormalImpulse :type "Vector Structure") (Hit :type "HitResult Structure (by ref)"))
  (`/Engine/EditorBlueprintResources/ActorMacros.Switch Has Authority`
    (:`Authority`
      (`self.spawnforall` Hit))
    (:`Remote`
      (`self.serverstuff` Hit))))

(event `spawnforall`
  (params (HitInfo :type "HitResult Structure (by ref)"))
  (bind _returnvalue (`SceneComponent.K2_GetComponentLocation` (`self.StaticMesh`)))
  (`KismetSystemLibrary.Delay` 3.0)
  (bind _returnvalue_2 (`GameplayStatics.SpawnEmitterAtLocation` "/Game/StarterContent/Particles/P_Explosion.P_Explosion" _returnvalue (struct) (5.0 5.0 5.0)))
  (`ActorComponent.SetIsReplicated` _returnvalue_2 true)
  (bind _returnvalue_3 (`|SpawnActorFromClass` "/Game/Blueprints/Gameplay/Burnmark.Burnmark_C" (`KismetMathLibrary.Conv_VectorToTransform` _returnvalue) "Undefined" "OverrideRootScale" null null))
  (`self.SetLifeSpan` _returnvalue_3 100.0)
  (`self.AddDamage`)
  (`KismetSystemLibrary.Delay` 0.2)
  (`self.K2_DestroyActor`))

(event `serverstuff`
  (params (HitInfo :type "HitResult Structure (by ref)"))
  (`self.spawnforall` HitInfo))

(event `AddDamage`
  (bind _sphere (`self.Sphere`))
  (bind _base_damage (`self.Base Damage`))
  (for _array_element (`PrimitiveComponent.GetOverlappingActors` _sphere "/Game/Blueprints/Characters/BaseCharacter.BaseCharacter_C")
    (bind _returnvalue (`self.K2_GetActorLocation` _array_element))
    (`GameplayStatics.ApplyPointDamage` _array_element (`KismetMathLibrary.FClamp` (- _base_damage (`KismetMathLibrary.Vector_Distance` (`SceneComponent.K2_GetComponentLocation` _sphere) _returnvalue)) 50.0 _base_damage) _returnvalue (stale `spawnforall` HitInfo) null self "/Engine/EngineDamageTypes/DmgTypeBP_Environmental.DmgTypeBP_Environmental_C")))

(fn `UserConstructionScript`
  (`ProjectileMovementComponent.SetVelocityInLocalSpace` (`self.ProjectileMovement`) (`self.New Velocity`)))